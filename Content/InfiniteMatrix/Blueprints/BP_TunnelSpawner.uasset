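; Spawner that builds a chain of BP_Tunnel segments, clearing existing ones at BeginPlay and laying the initial run from the player's location.
; Each new segment attaches at the newest tunnel's SpawnPoint, randomizes its wall and receives a spawner reference.
; Every segment also spawns a hidden Invisible_wall and either a random-chance health pack or, otherwise, an enemy given the player reference.
; Pickup and enemy offsets are randomized, and these extra actors expire on a timed lifespan.
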(event EventBeginPlay
  (CallFunction|SpawnInitialTunnels))

(event Collision|EventActorBeginOverlap
  (params (OtherActor :type Actor%20Object%20Reference)))

(event EventTick
  (params (DeltaSeconds :type Float%20%28single-precision%29)))

(fn ConstructionScript)

(fn SpawnTunnel
  (params (SpawnLocation :type Vector))
  (Utilities|FlowControl|Sequence
    (:then_0
      (bind _returnvalue (Game|SpawnActorfromClass "/Game/InfiniteMatrix/Blueprints/BP_Tunnel.BP_Tunnel_C" (Math|Transform|MakeTransform SpawnLocation "0, 0, 0" "1,1,1") "Undefined" 0 0))
      (bind _output_get (Variables|Default|SetNewestTunnel _returnvalue))
      (Variables|/Game/InfiniteMatrix/Blueprints/BP_Tunnel.BP_Tunnel_C|SetTunnelSpawner _output_get self)
      (Default|RandomizeWall _returnvalue))
    (:then_1
      (bind _createhealthpack (CallFunction|RandomizedHealthPack))
      (if _createhealthpack
        (bind _location (CallFunction|RandomizedHealthPackLocation))
        (bind _returnvalue_2 (Game|SpawnActorfromClass "/Game/InfiniteMatrix/Blueprints/HealthPack.HealthPack_C" (Math|Conversions|ToTransform(Vector) (+ SpawnLocation _location)) "Undefined" 0 0))
        (Actor|SetLifeSpan _returnvalue_2 3e+01)
        (else
          (CallFunction|RandomizedEnermy)
          (if true
            (bind _enermylocation (CallFunction|RandomizedEnermyLocation))
            (bind _returnvalue_3 (Game|SpawnActorfromClass "/Game/InfiniteMatrix/Blueprints/Enermy.Enermy_C" (Math|Conversions|ToTransform(Vector) (+ SpawnLocation _enermylocation)) "Undefined" 0 0 0))
            (Actor|SetLifeSpan _returnvalue_3 3e+01)
            (Variables|/Game/InfiniteMatrix/Blueprints/Enermy.Enermy_C|Setenermy_player _returnvalue_3 (Variables|Default|Getplayer))))))
    (:then_2
      (bind _returnvalue_4 (Game|SpawnActorfromClass "/Game/InfiniteMatrix/Blueprints/Invisible_wall.Invisible_wall_C" (Math|Conversions|ToTransform(Vector) SpawnLocation) "Undefined" 0 0))
      (Rendering|SetActorHiddenInGame _returnvalue_4 true)
      (Actor|SetLifeSpan _returnvalue_4 3e+01))))

(fn SpawnTunnelatSpawnPoint
  (CallFunction|SpawnTunnel (Transformation|GetWorldLocation (Variables|/Game/InfiniteMatrix/Blueprints/BP_Tunnel.BP_Tunnel_C|GetSpawnPoint (Variables|Default|GetNewestTunnel)))))

(fn SpawnInitialTunnels
  (bind _returnvalue (Game|Player|GetPlayerPawn 0))
  (Utilities|FlowControl|Sequence
    (:then_0
      (bind _outactors (Actor|GetAllActorsOfClass "/Game/InfiniteMatrix/Blueprints/BP_Tunnel.BP_Tunnel_C"))
      (for _array_element _outactors
        (Actor|DestroyActor _array_element)))
    (:then_1
      (for _index (range 0 2)
        (Utilities|IsValid (Variables|Default|GetNewestTunnel)
          (:Is%20Valid
            (CallFunction|SpawnTunnelatSpawnPoint))
          (:Is%20Not%20Valid
            (bind _asbp_player (Utilities|Casting|CastToBP_Player _returnvalue)
              (:then
                (Variables|Default|Setplayer _asbp_player)
                (CallFunction|SpawnTunnel (Transformation|GetActorLocation _returnvalue)))
              (:CastFailed
                (Development|PrintString "In BP Tunnel")))))))))

(fn RandomizedHealthPack
  (return (== 0 (Math|Random|RandomIntegerinRange 0 3))))

(fn RandomizedHealthPackLocation
  (switch int (Math|Random|RandomIntegerinRange 0 4)
    (:0
      (return (Math|Vector|MakeVector 0.0 2e+02 2e+02)))
    (:1
      (return (Math|Vector|MakeVector 0.0 -2e+02 -2e+02)))
    (:2
      (return (Math|Vector|MakeVector 0.0 -2e+02 2e+02)))
    (:3
      (return (Math|Vector|MakeVector 0.0 0.0 0.0)))))

(fn RandomizedHealthPackLocationTest
  (bind _returnvalue (Math|Random|RandomIntegerinRange 0 1))
  (if (== _returnvalue 0)
    (Development|PrintString "Hello")
    (elif (== _returnvalue 1)
      (Development|PrintString "Bye")
      (else
        (Development|PrintString "Bad")))))

(fn RandomizedEnermy
  (if (== (Math|Random|RandomIntegerinRange 0 0) 0)
    (return false)))

(fn RandomizedEnermyLocation
  (switch int (Math|Random|RandomIntegerinRange 0 4)
    (:0
      (return (Math|Vector|MakeVector 1.8e+03 1.5e+02 1.5e+02)))
    (:1
      (return (Math|Vector|MakeVector 1.8e+03 1.5e+02 -1.5e+02)))
    (:2
      (return (Math|Vector|MakeVector 1.8e+03 -1.5e+02 -1.5e+02)))
    (:3
      (return (Math|Vector|MakeVector 1.8e+03 0.0 0.0)))
    (:4
      (return (Math|Vector|MakeVector 1.8e+03 -1.5e+02 1.5e+02)))))